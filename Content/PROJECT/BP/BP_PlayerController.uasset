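; Player controller that turns Enhanced Input actions into camera switching and close-up commands for BP_CameraManager.
; BeginPlay adds the IMC_Camera mapping context.
; Left and right inputs step the camera number, gated by a delay-based cooldown and blocked during a close-up and briefly after leaving it.
; Enter and escape inputs toggle close-up state without checking either cooldown, printing debug strings like the other inputs.
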(event `self.ReceiveBeginPlay`
  ; Mappping
  (`EnhancedInputSubsystemInterface.AddMappingContext` (subsystem `EnhancedInputLocalPlayerSubsystem`) "/Game/PROJECT/Input/IMC_Camera.IMC_Camera" 0 (struct))
  (`KismetSystemLibrary.PrintString` "ControllerStarted"))

(event `EnhancedInput|/Game/PROJECT/Input/IA_CameraLeft`
  (params (ActionValue :type Boolean) (ElapsedSeconds :type "Float (double-precision)") (TriggeredSeconds :type "Float (double-precision)") (InputAction :type "InputAction Object Reference" :default "/Game/PROJECT/Input/IA_CameraLeft.IA_CameraLeft"))
  ; Rotate A D
  (:`Started`
    (if (`self.IsInCloseUp`)
      _
      (elif (`self.SwitchCooldown`)
        (if (not (`self.CloseUpCooldown`))
          (set `self.SwitchCooldown` false)
          (bind _returnvalue (`GameplayStatics.GetActorOfClass` "/Game/PROJECT/BP/BP_CameraManager.BP_CameraManager_C"))
          (`/Game/PROJECT/BP/BP_CameraManager.NextCameraNum` _returnvalue -1)
          (`KismetSystemLibrary.Delay` 0.6)
          (set `self.SwitchCooldown` true)
          (`KismetSystemLibrary.PrintString` "Left"))))))

(event `EnhancedInput|/Game/PROJECT/Input/IA_CameraRight`
  (params (ActionValue :type Boolean) (ElapsedSeconds :type "Float (double-precision)") (TriggeredSeconds :type "Float (double-precision)") (InputAction :type "InputAction Object Reference" :default "/Game/PROJECT/Input/IA_CameraRight.IA_CameraRight"))
  ; Rotate A D
  (:`Started`
    (if (`self.IsInCloseUp`)
      _
      (elif (`self.SwitchCooldown`)
        (if (not (`self.CloseUpCooldown`))
          (set `self.SwitchCooldown` false)
          (bind _returnvalue (`GameplayStatics.GetActorOfClass` "/Game/PROJECT/BP/BP_CameraManager.BP_CameraManager_C"))
          (`/Game/PROJECT/BP/BP_CameraManager.NextCameraNum` _returnvalue 1)
          (`KismetSystemLibrary.Delay` 0.6)
          (set `self.SwitchCooldown` true)
          (`KismetSystemLibrary.PrintString` "Right"))))))

(event `EnhancedInput|/Game/PROJECT/Input/IA_EnterCloseUp`
  (params (ActionValue :type Boolean) (ElapsedSeconds :type "Float (double-precision)") (TriggeredSeconds :type "Float (double-precision)") (InputAction :type "InputAction Object Reference" :default "/Game/PROJECT/Input/IA_EnterCloseUp.IA_EnterCloseUp"))
  ; Enter\Escape Closeup
  (:`Started`
    (if (not (`self.IsInCloseUp`))
      (set `self.CloseUpCooldown` true)
      (bind _returnvalue (`GameplayStatics.GetActorOfClass` "/Game/PROJECT/BP/BP_CameraManager.BP_CameraManager_C"))
      (`/Game/PROJECT/BP/BP_CameraManager.EnterCloseUp` _returnvalue)
      (set `self.IsInCloseUp` true)
      (`KismetSystemLibrary.Delay` 0.4)
      (set `self.CloseUpCooldown` true)
      (`KismetSystemLibrary.PrintString` "Enter"))))

(event `EnhancedInput|/Game/PROJECT/Input/IA_EscapeCloseUp`
  (params (ActionValue :type Boolean) (ElapsedSeconds :type "Float (double-precision)") (TriggeredSeconds :type "Float (double-precision)") (InputAction :type "InputAction Object Reference" :default "/Game/PROJECT/Input/IA_EscapeCloseUp.IA_EscapeCloseUp"))
  ; Enter\Escape Closeup
  (:`Started`
    (if (`self.IsInCloseUp`)
      (set `self.CloseUpCooldown` true)
      (bind _returnvalue (`GameplayStatics.GetActorOfClass` "/Game/PROJECT/BP/BP_CameraManager.BP_CameraManager_C"))
      (`/Game/PROJECT/BP/BP_CameraManager.EscapeCloseUp` _returnvalue)
      (set `self.IsInCloseUp` false)
      (`KismetSystemLibrary.Delay` 0.4)
      (set `self.CloseUpCooldown` false)
      (`KismetSystemLibrary.PrintString` "Escape"))))

(fn `UserConstructionScript`)