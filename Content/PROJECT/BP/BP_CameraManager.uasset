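; Camera manager that switches the player view between four station cameras: bed, transmitter, decrypt and tools.
; BeginPlay starts on the bed camera, and NextCameraNum steps the current index by a direction, wrapping at both ends.
; SwitchCamera moves player 0's view target to the selected camera with a short timed blend.
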(event `self.ReceiveBeginPlay`
  (`self.SwitchCamera` (`self.Camera0Bed`)))

(fn `NextCameraNum`
  (params (Direction :type Integer))
  (bind _currentcamera (`self.CurrentCamera`))
  (bind _output_get (set `self.CurrentCamera` (+ _currentcamera Direction)))
  (if (>= _output_get 4)
    (set `self.CurrentCamera` 0)
    (elif (< _output_get 0)
      (set `self.CurrentCamera` 3)))
  (switch `int` _currentcamera
    (:`0`
      (`self.SwitchCamera` (`self.Camera0Bed`)))
    (:`1`
      (`self.SwitchCamera` (`self.Camera1Transmitter`)))
    (:`2`
      (`self.SwitchCamera` (`self.Camera2Decrypt`)))
    (:`3`
      (`self.SwitchCamera` (`self.Camers3Tools`)))))

(fn `SwitchCamera`
  (params (TargetCamera :type "CameraActor Object Reference"))
  (`PlayerController.SetViewTargetWithBlend` (`GameplayStatics.GetPlayerController` 0) TargetCamera 0.5 "VTBlend_Linear" 0.0 false))

(fn `UserConstructionScript`)